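; Category actor with a player-facing title that expands into subcategory actors when overlapped.
; Its first overlap sends a VaRest GET request to the URL from BuildURL.
; A valid JSON response spawns a named SubCategories actor at a random nearby offset for each nested entry, then plays an explosion and destroys the category.
; Failed requests and invalid responses only print a message.
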(event Custom|OnSubCategoryComplete
  ;[1 1 1] API Processing - Load subcategories and destroy
  (if (Variables|/Script/VaRestPlugin.VaRestRequestJSON|GetbIsValidJsonResponse (Variables|Default|GetSubCategoryRequest))
    (bind _returnvalue (Class|VaRestRequestJSON|GetResponseObject (Variables|Default|GetSubCategoryRequest)))
    (bind _returnvalue_2 (Class|VaRestJsonObject|GetObjectArrayField _returnvalue "categories"))
    (for _array_element _returnvalue_2
      (bind _returnvalue_3 (Class|VaRestJsonObject|GetObjectArrayField _array_element "subCategories"))
      (for _array_element_2 _returnvalue_3
        (bind _returnvalue_4 (Game|SpawnActorfromClass "/Game/Blueprints/SubCategories.SubCategories_C" (Math|Transform|MakeTransform (+ (Math|Vector|MakeVector (Math|Random|RandomFloatinRange -1e+02 1e+02) (Math|Random|RandomFloatinRange -1e+02 1e+02) (Math|Random|RandomFloatinRange -2e+01 2e+01)) (Transformation|GetActorLocation))) false))
        (Rendering|Components|TextRender|SetText (Variables|/Game/Blueprints/SubCategories.SubCategories_C|GetTitle _returnvalue_4) (Class|VaRestJsonObject|GetStringField _array_element_2 "name"))))
    (Effects|SpawnEmitteratLocation "/Game/Particles/P_Explosion.P_Explosion" (Transformation|GetActorLocation))
    (Actor|DestroyActor)
    (else
      (Development|PrintString "Invalid JSON Response"))))

(event Custom|OnSubCategoryFail
  ;[1 1 1] API Processing - Load subcategories and destroy
  (Development|PrintString "Request failed!"))

(event EventActorBeginOverlap
  (params (OtherActor :type Actor%20Object%20Reference))
  (bind _returnvalue (|BuildURL))
  ;[1 1 1] API Processing - Load subcategories and destroy
  (Utilities|FlowControl|DoOnce false
    (:Completed
      (Variables|Default|SetSubCategoryRequest (Class|VaRestRequestJSON|ConstructRequestExt "GET" "x_www_form_urlencoded"))
      (EventDispatchers|BindEventtoOnRequestComplete (Variables|Default|GetSubCategoryRequest) (delegate Custom|OnSubCategoryComplete))
      (EventDispatchers|BindEventtoOnRequestFail (Variables|Default|GetSubCategoryRequest) (delegate Custom|OnSubCategoryFail))
      (Class|VaRestRequestJSON|ProcessURL (Variables|Default|GetSubCategoryRequest) _returnvalue)
      (Development|PrintString (Utilities|String|Append "Checking URL: " _returnvalue)))))

(event EventTick
  (params (DeltaSeconds :type Float%20%28single-precision%29))
  ;[1 1 1] Face Title Toward Player
  (Transformation|SetWorldRotation (Variables|Default|GetTitle) (Math|Rotator|MakeRotfromX (* (- (Transformation|GetWorldLocation (Variables|Default|GetTitle)) (Transformation|GetActorLocation (Game|GetPlayerCameraManager 0))) -1.0)) false))

(fn ConstructionScript)