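; SubCategories is a score pickup actor with a Title component that billboards toward the player camera every tick.
; When MyCharacter overlaps it, it adds a fixed bonus to the character's Score and passes the new total to MyHUD.
; It then plays a pitched-up cow moo at its location and destroys itself, but only if the HUD cast succeeds.
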(event EventTick
  (params (DeltaSeconds :type Float%20%28single-precision%29))
  (Utilities|FlowControl|Sequence
    (:then_0
      ;[1 1 1] Face Title Toward Character
      (Transformation|SetWorldRotation (Variables|Default|GetTitle) (Math|Rotator|MakeRotfromX (* (- (Transformation|GetWorldLocation (Variables|Default|GetTitle)) (Transformation|GetActorLocation (Game|GetPlayerCameraManager 0))) -1.0)) false))))

(event EventActorBeginOverlap
  (params (OtherActor :type Actor%20Object%20Reference))
  ;[1 1 1] Add to score and destroy
  (bind _asmycharacter_c (Utilities|Casting|CastToMyCharacter OtherActor))
  (Variables|/Game/Blueprints/MyCharacter.MyCharacter_C|SetScore _asmycharacter_c (+ (Variables|/Game/Blueprints/MyCharacter.MyCharacter_C|GetScore _asmycharacter_c) 100))
  (bind _asmyhud_c (Utilities|Casting|CastToMyHUD (HUD|GetHUD (Game|GetPlayerController 0))))
  (Default|UpdateScore _asmyhud_c (Variables|/Game/Blueprints/MyCharacter.MyCharacter_C|GetScore _asmycharacter_c))
  (Audio|PlaySoundatLocation "/Game/Audio/Cow_Moo-Mike_Koenig-42670858.Cow_Moo-Mike_Koenig-42670858" (Transformation|GetActorLocation) 1.0 2.0)
  (Actor|DestroyActor))

(fn ConstructionScript)