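; Spawn volume actor that fills its box with Categories actors built from categories fetched from a web API.
; BeginPlay and the MoreCategories input send a GET request to a built URL, with a DoOnce limiting it to once per press.
; Each JSON category spawns an actor at a random point within the box extent, carrying its name and ID.
; A successful response advances the page counter; failures only print messages.
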(event Custom|OnBaseCategoryComplete
  (bind _volume (Variables|Default|GetVolume))
  (bind _returnvalue (Components|Box|GetScaledBoxExtent _volume))
  (bind (_x _y _z) (Math|Vector|BreakVector _returnvalue))
  ;[1 1 1] Get Category identifiers
  (if (Variables|/Script/VaRestPlugin.VaRestRequestJSON|GetbIsValidJsonResponse (Variables|Default|GetCategoryRequest))
    (bind _returnvalue_2 (Class|VaRestRequestJSON|GetResponseObject (Variables|Default|GetCategoryRequest)))
    (bind _returnvalue_3 (Class|VaRestJsonObject|GetObjectArrayField _returnvalue_2 "categories"))
    (for _array_element _returnvalue_3
      (bind _returnvalue_4 (Game|SpawnActorfromClass "/Game/Blueprints/Categories.Categories_C" (Math|Transform|MakeTransform (+ (Math|Vector|MakeVector (Math|Random|RandomFloatinRange (* _x -1.0) _x) (Math|Random|RandomFloatinRange (* _y -1.0) _y) (Math|Random|RandomFloatinRange (* _z -1.0) _z)) (Transformation|GetActorLocation))) false))
      (Rendering|Components|TextRender|SetText (Variables|/Game/Blueprints/Categories.Categories_C|GetTitle _returnvalue_4) (Class|VaRestJsonObject|GetStringField _array_element "name"))
      (Variables|/Game/Blueprints/Categories.Categories_C|SetCategoryID _returnvalue_4 (Class|VaRestJsonObject|GetStringField _array_element "id")))
    (Variables|Default|SetPage (+ (Variables|Default|GetPage) 1))
    (else
      (Development|PrintString "Invalid JSON Response"))))

(event Custom|OnBaseCategoryFail
  ;[1 1 1] Get Category identifiers
  (Development|PrintString "Request failed!"))

(event EventBeginPlay
  (bind _returnvalue (|BuildingURL))
  ;[1 1 1] Get Category identifiers
  (Variables|Default|SetCategoryRequest (Class|VaRestRequestJSON|ConstructRequestExt "GET" "x_www_form_urlencoded"))
  (EventDispatchers|BindEventtoOnRequestComplete (Variables|Default|GetCategoryRequest) (delegate Custom|OnBaseCategoryComplete))
  (EventDispatchers|BindEventtoOnRequestFail (Variables|Default|GetCategoryRequest) (delegate Custom|OnBaseCategoryFail))
  (Class|VaRestRequestJSON|ProcessURL (Variables|Default|GetCategoryRequest) _returnvalue)
  (Development|PrintString (Utilities|String|Append "Checking URL: " _returnvalue)))

(event Input|ActionEvents|InputActionMoreCategories
  (bind _returnvalue (|BuildingURL))
  (:Pressed
    (Utilities|FlowControl|DoOnce false :!label _label
      (:Completed
        ;[1 1 1] Get Category identifiers
        (Class|VaRestRequestJSON|ProcessURL (Variables|Default|GetCategoryRequest) _returnvalue)
        (Development|PrintString (Utilities|String|Append "Checking URL: " _returnvalue)))))
  (:Released
    (goto _label Reset)))

(fn ConstructionScript)